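; BP_Monster is an enemy actor that penalizes or reacts to player contact through the game mode and dies to the axe.
; It caches FromWIthinGameMode on BeginPlay, calls CollideWithMonster on hitting BP_PlayerCharacter, and destroys itself when overlapping Axe_BP.
; InitMonster teleports it to a random spot at fixed height and re-arms a one-second timer on itself, though nothing in this Blueprint starts that loop.
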(event EventBeginPlay
  (bind _asfrom_within_game_mode (Utilities|Casting|CastToFromWIthinGameMode (Game|GetGameMode)))
  (Variables|Default|SetGameMode _asfrom_within_game_mode))

(event Collision|EventActorBeginOverlap
  (params (OtherActor :type Actor%20Object%20Reference))
  (Utilities|Casting|CastToAxe_BP OtherActor)
  (Actor|DestroyActor))

(event Collision|EventHit
  (params (MyComp :type Primitive%20Component%20Object%20Reference) (Other :type Actor%20Object%20Reference) (OtherComp :type Primitive%20Component%20Object%20Reference) (bSelfMoved :type Boolean) (HitLocation :type Vector :default "0, 0, 0") (HitNormal :type Vector :default "0, 0, 0") (NormalImpulse :type Vector :default "0, 0, 0") (Hit :type Hit%20Result%20Structure%20%28by%20ref%29))
  (Utilities|Casting|CastToBP_PlayerCharacter Other)
  (Default|CollidewithMonster (Variables|Default|GetGameMode)))

(fn ConstructionScript)

(fn InitMonster
  (Transformation|Teleport (Math|Vector|MakeVector (Math|Random|RandomFloatinRange -8e+01 2.3e+02) (Math|Random|RandomFloatinRange -1e+02 -2e+01) 1.3e+02) "0,-180.000000, 0")
  (Utilities|Time|SetTimerbyFunctionName 0 "InitMonster" 1.0))