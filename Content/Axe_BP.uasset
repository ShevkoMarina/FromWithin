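; Axe_BP is an axe item that the player can pick up into their inventory and use.
; On Interact, it adds its ItemInfo to the Inventory of BP_PlayerCharacter and destroys itself.
; On UseItem, it writes the same ItemInfo to PickedItem on FromWIthinGameMode, recording the picked item in the game mode.
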(event EventBeginPlay)

(event EventInteract
  (bind _asbp_player_character (Utilities|Casting|CastToBP_PlayerCharacter (Game|GetPlayerCharacter 0)))
  (Default|AddtoInventory (Variables|/Game/PlayerCharacter/BP_PlayerCharacter.BP_PlayerCharacter_C|GetInventory _asbp_player_character) (Variables|Default|GetItemInfo))
  (Actor|DestroyActor))

(event EventUseItem
  (bind _asfrom_within_game_mode (Utilities|Casting|CastToFromWIthinGameMode (Game|GetGameMode)))
  (Variables|/Game/FromWIthinGameMode.FromWIthinGameMode_C|SetPickedItem _asfrom_within_game_mode (Variables|Default|GetItemInfo)))

(event Collision|EventActorBeginOverlap
  (params (OtherActor :type Actor%20Object%20Reference)))

(event EventTick
  (params (DeltaSeconds :type Float%20%28single-precision%29)))

(fn ConstructionScript)